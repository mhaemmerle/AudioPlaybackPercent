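; BP_AudioTest is a test Blueprint that plays a sound and reports its playback progress.
; On BeginPlay it assigns SoundAsset to the Audio component, logs the sound's duration, binds the component's playback-percent and finished delegates, then plays from StartTime.
; The percent callback shows progress on screen only, with zero display duration, and the finished callback prints a completion message.
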(event `self.ReceiveBeginPlay`
  (bind _audio (`self.Audio`))
  (bind _audio_2 (`self.Audio`))
  (`AudioComponent.SetSound` _audio (`self.SoundAsset`))
  (`KismetSystemLibrary.PrintString` (`KismetTextLibrary.Conv_TextToString` (`|FormatText` "Duration in seconds: {duration}" (`SoundBase.Duration` (`AudioComponent.Sound` _audio)))) false)
  (add `AudioComponent.OnAudioPlaybackPercent` (`self.Audio`) (delegate `OnAudioPlaybackPercent_Event_1`))
  (add `AudioComponent.OnAudioFinished` _audio_2 (delegate `OnAudioFinished_Event_0`))
  (`AudioComponent.Play` _audio_2 (`self.StartTime`)))

(event `OnAudioFinished_Event_0`
  (`KismetSystemLibrary.PrintString` "Audio finished"))

(event `OnAudioPlaybackPercent_Event_1`
  (params (PlayingSoundWave :type "SoundWave Object Reference") (PlaybackPercent :type "Float (double-precision)"))
  (`KismetSystemLibrary.PrintString` (`KismetTextLibrary.Conv_TextToString` (`|FormatText` "{Percent} %" PlaybackPercent)) true false (struct :`G` 0.66 :`B` 1.0 :`A` 1.0) 0.0))

(fn `UserConstructionScript`)